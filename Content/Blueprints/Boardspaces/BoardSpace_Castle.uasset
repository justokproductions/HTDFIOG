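; BoardSpace_Castle is the castle variant of a board space, derived from a parent Blueprint.
; It adds no logic of its own: mouse-over, not-selectable, BeginPlay, selection-fly generation and update, and construction each only call the parent implementation.
; Overlap and Tick are disabled stubs, so any castle-specific difference lies outside these graphs.
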(event EventBeginPlay
  (|CallParentFunction))

(event Collision|EventActorBeginOverlap
  (params (OtherActor :type Actor%20Object%20Reference)))

(event EventTick
  (params (DeltaSeconds :type Float%20%28single-precision%29)))

(event EventMousedOveron
  (|CallParentFunction))

(event EventMousedOverOff
  (|CallParentFunction))

(event EventNotSelectable
  (|CallParentFunction))

(event EventGenerateSelectionFlies
  (|CallParentFunction))

(event EventUpdateSelectionFlies
  (params (Color :type Linear%20Color%20Structure) (Size :type Float%20%28single-precision%29))
  (|CallParentFunction Color Size))

(fn ConstructionScript
  (|CallParentFunction))