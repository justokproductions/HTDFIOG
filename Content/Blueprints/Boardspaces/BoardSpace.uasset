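; Board game space actor that tracks the pieces on it and shows whether it can be selected as a move destination.
; MovementCheck recurses through adjacent spaces except the previous one, spending movement points and accumulating path and animations.
; When a neighbor is unaffordable, the current space becomes selectable and stores its path.
; Selection and hover states recolor SelectionLight; firefly spawning is disconnected and the encounter check always returns true.
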(event Custom|MousedOverOn
  ;[1 1 1] Updates the Board Space based on if it is selectable or not
  (CallFunction|UpdateSelectionFlies (Variables|FireflyValues|GetColorHighlighted) 5e+03))

(event Custom|MousedOverOff
  ;[1 1 1] Updates the Board Space based on if it is selectable or not
  (CallFunction|UpdateSelectionFlies (Variables|FireflyValues|GetColorSelectable) 5e+03))

(event Custom|NotSelectable
  ;[1 1 1] Updates the Board Space based on if it is selectable or not
  (CallFunction|UpdateSelectionFlies (Variables|FireflyValues|GetColorUnselectable) (Variables|FireflyValues|GetSizeUnselectable)))

(event EventBeginPlay
  (Variables|FireflyValues|SetSizeSelectable 2.0)
  (Variables|FireflyValues|SetColorSelectable "(R=0.000000,G=0.822435,B=1.000000,A=1.000000)")
  (CallFunction|GenerateSelectionFlies))

(event EventTick
  (params (DeltaSeconds :type Float%20%28single-precision%29)))

(fn ConstructionScript)

(fn GenerateSelectionFlies)

(fn UpdateSelectionFlies
  (params (Color :type Linear%20Color%20Structure) (Size :type Float%20%28single-precision%29))
  (bind _selectionlight (Variables|Default|GetSelectionLight))
  (Rendering|Components|Light|SetIntensity _selectionlight Size)
  (Rendering|Components|Light|SetLightColor _selectionlight Color true))

(fn MovementCheck
  (params (Movement :type Integer) (PathIn :type Array%20of%20Board%20Space%20Object%20References) (MovementIn :type Array%20of%20AnimTypes%20Enums :default "NewEnumerator0") (FirstSpace :type Boolean) (PreviousSpace :type Board%20Space%20Object%20Reference) (MoveFromPrev :type AnimTypes%20Enum :default "NewEnumerator0"))
  (bind _adjacentspaces (Variables|Default|GetAdjacentSpaces))
  ;[1 1 1] Sets the path so far, and checks if this is the first space.
  (LocalVariables|SetRemainingMovePoints Movement)
  (LocalVariables|SetPathSoFar PathIn)
  (LocalVariables|SetAnimationSoFar MovementIn)
  (LocalVariables|SetPrevious PreviousSpace)
  (if FirstSpace
    ;[1 1 1] First space does not take up movement points, so skips movement checks, boosts the Remaining Move Points number to avoid fall off later
    (LocalVariables|SetRemainingMovePoints (+ (LocalVariables|GetRemainingMovePoints) (Variables|Default|GetSpaceCost)))
    ;[1 1 1] Goes through each of the following spaces and recurses the function.  If it's the last space, than it becomes selectable.
    (for (_array_element _array_index) _adjacentspaces :!label _label
      (if (!= _array_element (LocalVariables|GetPrevious))
        (bind _endpath (CallFunction|MovementCheck _array_element (- (LocalVariables|GetRemainingMovePoints) (Variables|Default|GetSpaceCost)) (LocalVariables|GetPathSoFar) (LocalVariables|GetAnimationSoFar) false self (Utilities|Array|Get(acopy) (Variables|Default|GetAdjacentAnims) _array_index)))
        (if _endpath
          (Variables|Default|SetSelectable? true)
          (CallFunction|MousedOverOff)
          (Variables|Default|SetListofPaths (LocalVariables|GetPathSoFar)))))
    (return false)
    (else
      ;[1 1 1] Checks if the player can move to this space. Adds to the path if viable
      (if (>= (LocalVariables|GetRemainingMovePoints) (Variables|Default|GetSpaceCost))
        (Utilities|Array|Add (LocalVariables|GetPathSoFar) self)
        (Utilities|Array|Add (LocalVariables|GetAnimationSoFar) MoveFromPrev)
        (if (> (Utilities|Array|Length _adjacentspaces) 0)
          (goto _label))
        (else
          (return true))))))

(fn AddPlayersonSpace
  (params (CurrentPiece :type 00%20Base%20Object%20Reference))
  (Utilities|Array|AddUnique (Variables|Default|GetPlayersOnSpace) CurrentPiece))

(fn RemovePlayeronSpace
  (params (CurrentPiece :type 00%20Base%20Object%20Reference))
  (Utilities|Array|RemoveItem (Variables|Default|GetPlayersOnSpace) CurrentPiece))

(fn ClearSelection
  (Variables|Default|SetSelectable? false)
  (CallFunction|NotSelectable)
  (Utilities|Array|Clear (Variables|Default|GetListofPaths)))

(fn CheckforExistingEncounters
  (return true))