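; Base character Blueprint with modular body and gear meshes that follow the main skeletal mesh through master pose.
; SetAnimation switches between Run, Jump and Idle clips without an anim graph.
; Movetospace moves the capsule to a target with MoveComponentTo; in Jump, Tick stops that move once MoveDuration elapses, using a cosine Z offset.
; JumpMotions plays the landing clip but is not called here.
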(event Custom|Move%20to%20space
  (params (Target%20Location :type Vector) (TargetRelativeRotation :type Rotator))
  (bind (_x _y _z) (Math|Vector|BreakVector Target%20Location))
  (bind _capsulecomponent (Variables|Collision|GetCapsuleComponent))
  (switch Utilities|FlowControl|Switch|SwitchonAnimTypes (Variables|Default|GetCurrentAnim)
    (:NewEnumerator0
      _)
    (:NewEnumerator1
      (Components|MoveComponentTo _capsulecomponent (Math|Vector|MakeVector _x _y (+ _z (* (Math|Trig|Cos(Degrees) (* (/ (Variables|Default|GetTimeSoFar) (Variables|Default|GetMoveDuration)) 9e+01)) 4e+02))) TargetRelativeRotation false false 0.4 false)))
  (Components|MoveComponentTo _capsulecomponent Target%20Location TargetRelativeRotation false false 0.2 false))

(event EventBeginPlay
  (Class|SkinnedMeshComponent|SetMasterPoseComponent (Variables|Default|GetHair) (Variables|Default|GetSkeletalMesh) false))

(event Collision|EventActorBeginOverlap
  (params (OtherActor :type Actor%20Object%20Reference)))

(event EventTick
  (params (DeltaSeconds :type Float%20%28single-precision%29))
  (bind _capsulecomponent (Variables|Collision|GetCapsuleComponent))
  (switch Utilities|FlowControl|Switch|SwitchonAnimTypes (Variables|Default|GetCurrentAnim)
    (:NewEnumerator1
      (bind _output_get (Variables|Default|SetTimeSoFar (+ (Variables|Default|GetTimeSoFar) DeltaSeconds)))
      (if (not (<= _output_get (Variables|Default|GetMoveDuration)))
        (Components|MoveComponentTo _capsulecomponent (Math|Vector|MakeVector (.X (Math|Vector|BreakVector (stale Custom|Move%20to%20space Target%20Location))) (.Y (Math|Vector|BreakVector (stale Custom|Move%20to%20space Target%20Location))) (+ (.Z (Math|Vector|BreakVector (stale Custom|Move%20to%20space Target%20Location))) (* (Math|Trig|Cos(Degrees) (* (/ (Variables|Default|GetTimeSoFar) (Variables|Default|GetMoveDuration)) 9e+01)) 4e+02))) (stale Custom|Move%20to%20space TargetRelativeRotation) false false 0.4 false) ; enters at Stop
      ))))

(fn ConstructionScript)

(fn SetAnimation
  (params (Animation :type AnimTypes%20Enum :default "NewEnumerator0"))
  (bind _skeletalmesh (Variables|Default|GetSkeletalMesh))
  (bind _skeletalmesh_2 (Variables|Default|GetSkeletalMesh))
  (bind _skeletalmesh_3 (Variables|Default|GetSkeletalMesh))
  (bind _output_get (Variables|Default|SetCurrentAnim Animation))
  (switch Utilities|FlowControl|Switch|SwitchonAnimTypes _output_get
    (:NewEnumerator0
      (Components|Animation|SetAnimation _skeletalmesh_2 "/Game/ModularRPGHeroesPolyart/Animations/NoWeaponStance/NormalRun_noWeaponAnim.NormalRun_noWeaponAnim")
      (Audio|Components|Audio|Play _skeletalmesh_2 true))
    (:NewEnumerator1
      (Components|Animation|SetAnimation _skeletalmesh_3 "/Game/ModularRPGHeroesPolyart/Animations/NoWeaponStance/JumpStart_noWeaponAnim.JumpStart_noWeaponAnim")
      (Audio|Components|Audio|Play _skeletalmesh_3 false)
      (Variables|Default|SetTimeSoFar 0.0))
    (:NewEnumerator2
      (Components|Animation|SetAnimation _skeletalmesh "/Game/ModularRPGHeroesPolyart/Animations/NoWeaponStance/Idle_noWeaponAnim.Idle_noWeaponAnim")
      (Audio|Components|Audio|Play _skeletalmesh true))))

(fn JumpMotions
  (params (delta :type Float%20%28single-precision%29))
  (bind _skeletalmesh (Variables|Default|GetSkeletalMesh))
  (Variables|Default|SetTimeSoFar (+ (Variables|Default|GetTimeSoFar) delta))
  (if (not (Audio|Components|Audio|IsPlaying (Variables|Default|GetSkeletalMesh)))
    (Components|Animation|SetAnimation _skeletalmesh "/Game/ModularRPGHeroesPolyart/Animations/NoWeaponStance/JumpEnd_noWeaponAnim.JumpEnd_noWeaponAnim")
    (Audio|Components|Audio|Play _skeletalmesh false)
    (Development|PrintString "Juimp")))