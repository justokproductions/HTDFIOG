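; HeroWhite is a hero character Blueprint assembled from modular mesh parts such as hair, gloves, shoes, headgear, shoulder pads, belt and face.
; On BeginPlay it sets the main SkeletalMesh as master pose component for each part, so they all follow one skeleton's animation.
; A Movetospace custom event uses MoveComponentTo to move the capsule to a given target relative location.
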(event Custom|Move%20to%20space
  (params (Target%20Location :type Vector))
  (Components|MoveComponentTo (Variables|Collision|GetCapsuleComponent) Target%20Location "0, 0, 0" false false 0.2 false))

(event EventBeginPlay
  (Class|SkinnedMeshComponent|SetMasterPoseComponent (Variables|Default|GetHair) (Variables|Default|GetSkeletalMesh) false))

(event Collision|EventActorBeginOverlap
  (params (OtherActor :type Actor%20Object%20Reference)))

(event EventTick
  (params (DeltaSeconds :type Float%20%28single-precision%29)))

(fn ConstructionScript)