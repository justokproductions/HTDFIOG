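; A card Blueprint for the "Run" card 01, one specific set of movement, attack and defense stats with its own face texture.
; On BeginPlay it calls the parent, then writes its stats, movement type and texture into variables.
; It adds no other behavior: overlap and tick events are disabled, and the construction script only calls the parent.
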(event EventBeginPlay
  (|CallParentFunction)
  (Variables|Default|SetMovement 6)
  (Variables|Default|SetMovementType "NewEnumerator0")
  (Variables|Default|SetAttack 2)
  (Variables|Default|SetDefense 2)
  (Variables|Default|SetFaceTexture "/Game/Textures/CardImages/01_Run_6_2_2.01_Run_6_2_2"))

(event Collision|EventActorBeginOverlap
  (params (OtherActor :type Actor%20Object%20Reference))
  (|CallParentFunction OtherActor) ; This node is disabled and will not be called.\nDrag off pins to build functionality.
)

(event EventTick
  (params (DeltaSeconds :type Float%20%28single-precision%29))
  (|CallParentFunction DeltaSeconds) ; This node is disabled and will not be called.\nDrag off pins to build functionality.
)

(fn ConstructionScript
  (|CallParentFunction))