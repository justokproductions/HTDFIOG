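; Deck actor that manages a player's draw pile, hand and discard pile of cards.
; StartingDeck fills the pile with references to level-placed 00_Card actors, some repeated, then shuffles and draws the starting hand.
; DrawCard reshuffles the discard when empty, refreshes the owner's chat widget and can start movement using the drawn card's Movement.
; PlayCard moves the chosen hand card to the discard.
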(event EventBeginPlay)

(event Collision|EventActorBeginOverlap
  (params (OtherActor :type Actor%20Object%20Reference)))

(event EventTick
  (params (DeltaSeconds :type Float%20%28single-precision%29)))

(fn ConstructionScript)

(fn StartingDeck
  (bind _outactors (Actor|GetAllActorsOfClass "/Game/Blueprints/Cards/IndividualCards/00_Card.00_Card_C"))
  (bind _output_get (Variables|Locations|SetDrawPile (Utilities|Array|MakeArray (Utilities|Array|Get(acopy) _outactors) 0 (Utilities|Array|Get(acopy) _outactors 1) (Utilities|Array|Get(acopy) _outactors 1) (Utilities|Array|Get(acopy) _outactors 2) (Utilities|Array|Get(acopy) _outactors 2) (Utilities|Array|Get(acopy) _outactors 3) (Utilities|Array|Get(acopy) _outactors 4) (Utilities|Array|Get(acopy) _outactors 5))))
  (Utilities|Array|Shuffle _output_get)
  (for _index (range 1 (Variables|Default|GetStartingHandSize))
    (Locations|DrawCard false)))

(fn DrawCard
  (params (MovePhase? :type Boolean))
  (bind _owningplayer (Variables|Default|GetOwningPlayer))
  (bind _drawpile (Variables|Locations|GetDrawPile))
  (bind _output (Utilities|Array|Get(acopy) _drawpile))
  ;[1 1 1] If there's no draw pile, shuffle the discard into the draw.  If there's neither, than no draw is possible.
  (if (<= (Utilities|Array|Length _drawpile) 0)
    (bind _success (Locations|ShuffleDiscard))
    (if _success
      _
      (else
        (return false))))
  ;[1 1 1] Pulls a card out of the draw pile and into the hand.  Updates the WB
  (LocalVariables|SetNewCard _output)
  (Utilities|Array|Add (Variables|Locations|GetHand) _output)
  (Utilities|Array|RemoveIndex (Variables|Locations|GetDrawPile))
  (Utilities|IsValid (Variables|/Game/Blueprints/Gameplay/GameplayPC.GameplayPC_C|GetGameplayChatWB (Variables|Default|GetOwningPlayer))
    (:Is%20Valid
      _)
    (:Is%20Not%20Valid
      (Development|PrintString (Utilities|String|Append (Utilities|GetDisplayName _owningplayer) ": " (Utilities|GetDisplayName (Variables|/Game/Blueprints/Gameplay/GameplayPC.GameplayPC_C|GetGameplayChatWB _owningplayer))) true true "(R=1.000000,G=0.894773,B=0.000000,A=1.000000)" 2e+01)
      (Default|SetupChatWindow (Variables|Default|GetOwningPlayer))))
  (Default|CollectHandData (Variables|/Game/Blueprints/Gameplay/GameplayPC.GameplayPC_C|GetGameplayChatWB (Variables|Default|GetOwningPlayer)))
  ;[1 1 1] If this card was drawn as part of the movement phase, than find the possible directions
  (if MovePhase?
    (Default|MovePhase (Variables|Default|GetOwningPlayer) (Variables|/Game/Blueprints/Cards/IndividualCards/00_Card.00_Card_C|GetMovement (LocalVariables|GetNewCard)))
    (Variables|/Game/Blueprints/Gameplay/GameplayPC.GameplayPC_C|SetTurnPhase (Variables|Default|GetOwningPlayer) "NewEnumerator2")
    (return true)
    (else
      (return true))))

(fn ShuffleDiscard
  (bind _discard (Variables|Locations|GetDiscard))
  ;[1 1 1] Move the Discard back into the Deck, clear the discard, and then shuffle. If the discard is empty, pass back a failure.
  (if (> (Utilities|Array|Length (Variables|Locations|GetDiscard)) 0)
    (bind _output_get (Variables|Locations|SetDrawPile _discard))
    (Utilities|Array|Clear _discard)
    (Utilities|Array|Shuffle _output_get)
    (return true)
    (else
      (return false))))

(fn PlayCard
  (params (CardNumber :type Integer))
  (LocalVariables|SetHandIndex CardNumber)
  (Development|PrintString (Utilities|String|Append "Card played: " (Utilities|GetDisplayName (Utilities|Array|Get(acopy) (Variables|Locations|GetHand) (LocalVariables|GetHandIndex)))))
  (Utilities|Array|Add (Variables|Locations|GetDiscard) (Utilities|Array|Get(acopy) (Variables|Locations|GetHand) (LocalVariables|GetHandIndex)))
  (Utilities|Array|RemoveIndex (Variables|Locations|GetHand) (LocalVariables|GetHandIndex))
  (return true))