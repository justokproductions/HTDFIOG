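; Game state for a turn-based multiplayer board game, tracking players, turn order, the current turn and the current combat.
; Each new player rebuilds the turn order cards; once every piece has drawn one, it sorts pieces and controllers together and starts the game on each controller.
; It cycles turns, relays movement cards and turn phases to all controllers, and spawns combat data actors.
; SetCurrentTurn sets MyTurn false on both branches.
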(event Custom|Get%20Ready%20Value
  (params (ItemToFind :type 00%20Base%20Class%20Reference%20%28by%20ref%29)))

(event Custom|Draw%20Turn%20Order%20Card
  (params (Selected%20Card :type Integer) (ControlledPiece :type 00%20Base%20Object%20Reference))
  (bind _turnordercards (Variables|Default|GetTurnOrderCards))
  (Variables|/Game/Blueprints/Characters/00_Base.00_Base_C|SetTurnOrder ControlledPiece (Utilities|Array|Get(acopy) _turnordercards Selected%20Card))
  (Utilities|Array|SetArrayElem _turnordercards Selected%20Card 0)
  (CallFunction|CheckAllReady))

(event Custom|SetCurrentCombat
  (params (CurrentCombat :type Combatdata%20Object%20Reference))
  (Variables|Default|SetCurrentCombat CurrentCombat))

(event Custom|SpawnCombat
  (bind _returnvalue (Game|SpawnActorfromClass "/Game/Blueprints/CombatZones/Combatdata.Combatdata_C" (Math|Transform|MakeTransform "0, 0, 0") "Undefined" 0 0))
  (CallFunction|SetCurrentCombat _returnvalue))

(event EventBeginPlay)

(event EventTick
  (params (DeltaSeconds :type Float%20%28single-precision%29)))

(fn ConstructionScript)

(fn AddNewPlayer
  (params (NewItem :type Gameplay%20PC%20Object%20Reference%20%28by%20ref%29))
  (bind _returnvalue (Utilities|Array|AddUnique (Variables|Default|GetAllPlayerControllers) NewItem))
  (if (>= _returnvalue 0)
    (Math|Integer|IncrementInt (Variables|Default|GetNumberOfPlayers)
      (:%20%20
        (Utilities|Array|Clear (Variables|Default|GetTurnOrderCards))
        (for _index (range 1 (Variables|Default|GetNumberOfPlayers))
          (Utilities|Array|Add (Variables|Default|GetTurnOrderCards) _index))))))

(fn CheckAllReady
  (LocalVariables|SetReady? true)
  (bind _array_element (Utilities|Array|ForEachLoopwithBreak (Variables|Default|GetAllPlayerPieces) :!label _label)
    (:LoopBody
      (if (not (> (Variables|/Game/Blueprints/Characters/00_Base.00_Base_C|GetTurnOrder _array_element) 0))
        (LocalVariables|SetReady? false)
        (goto _label Break)))
    (:Completed
      (if (LocalVariables|GetReady?)
        (Development|PrintString "Ready!")
        (CallFunction|GameStartup)
        (else
          (Development|PrintString "Not Ready"))))))

(fn GameStartup
  (CallFunction|RearrangeTurnOrder)
  (for _array_element (Variables|Default|GetAllPlayerControllers)
    (Default|ChangeSwitchClient _array_element 1)
    (Default|StartingDeckClient _array_element)
    (Default|SetMyTurn _array_element)))

(fn RearrangeTurnOrder
  (bind _allplayerpieces (Variables|Default|GetAllPlayerPieces))
  (bind _allplayerpieces_2 (Variables|Default|GetAllPlayerPieces))
  (for (_ _array_index) _allplayerpieces
    (for _index (range (+ _array_index 1) (- (Utilities|Array|Length _allplayerpieces) 1))
      (if (> (Variables|/Game/Blueprints/Characters/00_Base.00_Base_C|GetTurnOrder (Utilities|Array|Get(acopy) _allplayerpieces_2 _array_index)) (Variables|/Game/Blueprints/Characters/00_Base.00_Base_C|GetTurnOrder (Utilities|Array|Get(acopy) _allplayerpieces_2 _index)))
        (Utilities|Array|Swap (Variables|Default|GetAllPlayerPieces) _index _array_index)
        (Utilities|Array|Swap (Variables|Default|GetAllPlayerControllers) _array_index _index)))))

(fn MovetoNextTurn
  (if (>= (Variables|Default|GetCurrentTurn) (Utilities|Array|Length (Variables|Default|GetAllPlayerPieces)))
    (Variables|Default|SetCurrentTurn 1)
    (else
      (Math|Integer|IncrementInt (Variables|Default|GetCurrentTurn)
        (:%20%20
          _))))
  (Development|PrintString (Utilities|String|Append "Move to turn # " (Utilities|String|ToString(Integer) (Variables|Default|GetCurrentTurn))) true true "(R=0.000000,G=1.000000,B=0.312809,A=1.000000)"))

(fn SeeMovementCard
  (params (NewCard :type 00%20Player%20Cards%20Object%20Reference))
  (bind _currentturn (Variables|Default|GetCurrentTurn))
  (for _array_element (Variables|Default|GetAllPlayerControllers)
    (Development|PrintString (Utilities|String|Append (Utilities|GetDisplayName _array_element) " (" (Utilities|String|ToString(Integer) (Variables|/Game/Blueprints/Characters/00_Base.00_Base_C|GetTurnOrder (Variables|/Game/Blueprints/Gameplay/GameplayPC.GameplayPC_C|GetPlayerPiece _array_element))) ") ?= " (Utilities|String|ToString(Integer) _currentturn)) true true "(R=0.916354,G=0.000000,B=1.000000,A=1.000000)" 22.0)
    (if (!= (Variables|/Game/Blueprints/Characters/00_Base.00_Base_C|GetTurnOrder (Variables|/Game/Blueprints/Gameplay/GameplayPC.GameplayPC_C|GetPlayerPiece _array_element)) _currentturn)
      _
      (else
        _))
    (Default|GenerateCardRemote _array_element NewCard)))

(fn SetTurnPhase
  (params (TurnPhase :type TurnPhases%20Enum :default "NewEnumerator0"))
  (for _array_element (Variables|Default|GetAllPlayerControllers)
    (Default|SetTurnPhaseRemote _array_element TurnPhase)))

(fn GetCurrentCombat
  (return (Variables|Default|GetCurrentCombat)))