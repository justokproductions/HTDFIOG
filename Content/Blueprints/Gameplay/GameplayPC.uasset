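; Player controller for a turn-based multiplayer board and card game with monster combat.
; On local start it loads the saved player info for GameplayGM to spawn the character and sets up the chat and hand widget.
; It manages deck, hand, discard and combat card slots, while turn phases drive cursor highlighting and click-to-move on BoardSpaces.
; Pathing, movement, combat and turn endings route through GameplayGM; death is a stub and debug keys remain.
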(event Custom|PassCharacterInfoToServer
  (params (PlayerInfoSettings :type Player%20Info%20Structure))
  ;[1 1 1] Passes in Player Info / Spawns player / loads chat window
  (Variables|Default|SetPlayerSettings PlayerInfoSettings)
  (bind _asgameplay_gm (Utilities|Casting|CastToGameplayGM (Game|GetGameMode)))
  (Default|RespawnPlayer _asgameplay_gm self (.MyPlazyerCharacter (Utilities|Struct|BreakPlayerInfo (Variables|Default|GetPlayerSettings))))
  (CallFunction|SetupChatWindow))

(event Custom|SetupChatWindow
  ;[1 1 1] Creates Chat
  (bind _returnvalue (UserInterface|CreateWidget "/Game/UI/AllLevels/GameplayMenu.GameplayMenu_C"))
  (bind _output_get (Variables|Default|SetGameplayChatWB _returnvalue))
  (UserInterface|Viewport|AddtoViewport _output_get 0))

(event Custom|Update%20Camera%20Remote)

(event Custom|AssignPiece
  (params (PlayerPiece :type 00%20Base%20Object%20Reference))
  (Variables|Default|SetPlayerPiece PlayerPiece))

(event Custom|UpdateChat
  (params (SenderName :type Text) (SenderText :type Text))
  ;[1 1 1] Processes new messages and calls update chat
  (Default|UpdateChatWindow (Variables|/Game/UI/AllLevels/GameplayMenu.GameplayMenu_C|GetGameplayChat (Variables|Default|GetGameplayChatWB)) SenderName SenderText))

(event Custom|Change%20Camera
  (params (NewViewTarget :type Actor%20Object%20Reference))
  (bind _outactors (Actor|GetAllActorsOfClass "/Game/Blueprints/CombatZones/CombatZone_Blueprint.CombatZone_Blueprint_C"))
  (Game|Player|SetViewTargetwithBlend (Utilities|Array|Get(acopy) _outactors) 0.0 "VTBlend_Linear" 1.0 true)
  (Development|PrintString (Utilities|String|ToString(Integer) (Utilities|Array|Length _outactors))))

(event Custom|AddPlayer
  (Default|AddPlayer (Utilities|GetGameplayGM) self))

(event Custom|EndTurn
  ;[1 1 1] Calls End Turn mechanic on Server
  (Default|EndTurn (Utilities|GetGameplayGM)))

(event Custom|ReplicateCombatResolve
  (params (TargetMonster :type Integer))
  (bind (_bothcard _attackcard _defensecard) (Utilities|CardOptions))
  (Utilities|IsValid _bothcard
    (:Is%20Valid
      (Default|CombatResolve (Utilities|GetGameplayGM) _bothcard _bothcard TargetMonster))
    (:Is%20Not%20Valid
      (Default|CombatResolve (Utilities|GetGameplayGM) _attackcard _defensecard TargetMonster))))

(event Custom|Update%20Cards
  (Default|CollectHandData (Variables|Default|GetGameplayChatWB)))

(event Custom|GetChatMessage
  (params (TextToSend :type Text))
  ;[1 1 1] Processes new messages and calls update chat
  (Variables|Default|SetSenderText TextToSend)
  (Variables|Default|SetSenderName (.MyPlayerName (Utilities|Struct|BreakPlayerInfo (Variables|Default|GetPlayerSettings))))
  (for _array_element (Variables|/Game/Blueprints/Gameplay/GameplayGM.GameplayGM_C|GetAllPlayerControllers (.AsGameplay%20GM (Utilities|Casting|CastToGameplayGM (Game|GetGameMode))))
    (bind _asgameplay_pc (Utilities|Casting|CastToGameplayPC _array_element))
    (CallFunction|UpdateChat _asgameplay_pc (Variables|Default|GetSenderName) (Variables|Default|GetSenderText))))

(event EventBeginPlay
  (if (Pawn|IsLocalController)
    ;[1 1 1] Loads character info on the server
    (Viewport|RemoveAllWidgets)
    (CallFunction|LoadGame)
    (Utilities|FlowControl|Delay 0.0)
    (CallFunction|PassCharacterInfotoServer (Variables|Default|GetPlayerSettings))
    (CallFunction|AddPlayer)
    (CallFunction|InitialTurnPhase)
    (CallFunction|UpdateCameraRemote)
    (Default|CommitReady (Variables|Default|GetPlayerPiece))))

(event EventTick
  (params (DeltaSeconds :type Float%20%28single-precision%29))
  (bind _hitresult (Game|Player|GetHitResultUnderCursorbyChannel "TraceTypeQuery1" true))
  (bind _hitactor (Collision|BreakHitResult _hitresult))
  (CallFunction|DisplayTest)
  (switch Utilities|FlowControl|Switch|SwitchonTurnPhases (Variables|Default|GetTurnPhase)
    (:NewEnumerator2
      ;[1 1 1] Checks what is being moused over and updates all information appropriately
      (Utilities|FlowControl|Sequence
        (:then_0
          ;;[1 1 1] Checks if moving off of a selectable object and adjusts appropriately
          (if (not (== _hitactor (Variables|Default|GetSelectedSpace))) ; Checks if matches previous
            (if (not (== (Variables|Default|GetSelectedSpace) 0)) ; Checks if previous was null
              (bind _asboard_space (Utilities|Casting|CastToBoardSpace (Variables|Default|GetSelectedSpace)))
              (if (Variables|/Game/Blueprints/Boardspaces/BoardSpace.BoardSpace_C|GetSelectable? _asboard_space)
                (Default|MousedOverOff _asboard_space)))))
        (:then_1
          ;;[1 1 1] Checks if highlighting a new selectable object
          (bind _asboard_space_2 (Utilities|Casting|CastToBoardSpace _hitactor))
          (if (Variables|/Game/Blueprints/Boardspaces/BoardSpace.BoardSpace_C|GetSelectable? _asboard_space_2)
            (Default|MousedOveron _asboard_space_2)))
        (:then_2
          ;;[1 1 1] Updates previous selection
          (Variables|Default|SetSelectedSpace _hitactor))))
    (:NewEnumerator3
      (CallFunction|ServerPieceMove))))

(event Input|KeyboardEvents|T
  (params (Key :type Key%20Structure :default "None"))
  ;[1 1 1] Processes new messages and calls update chat
  (:Pressed
    (bind _isa (Utilities|FlowControl|FlipFlop)
      (:A
        _)
      (:B
        _))
    (Variables|Default|SetbShowMouseCursor _isa)))

(event Input|MouseEvents|LeftMouseButton
  (params (Key :type Key%20Structure :default "None"))
  ;[1 1 1] Allows player to move to selected location
  (:Pressed
    (Utilities|IsMyTurn?
      (:Yes
        (bind _asboard_space (Utilities|Casting|CastToBoardSpace (.HitActor (Collision|BreakHitResult (.HitResult (Game|Player|GetHitResultUnderCursorbyChannel "TraceTypeQuery1" true))))))
        (if (Variables|/Game/Blueprints/Boardspaces/BoardSpace.BoardSpace_C|GetSelectable? _asboard_space)
          (CallFunction|ServerPieceMovementPath (Variables|/Game/Blueprints/Boardspaces/BoardSpace.BoardSpace_C|GetListofPaths _asboard_space))
          (Variables|Default|SetTurnPhase "NewEnumerator3"))))))

(fn ConstructionScript)

(fn LoadGame
  (bind _returnvalue (SaveGame|LoadGamefromSlot (LocalVariables|GetPlayerSettingsSave)))
  (bind _asplayer_save (Utilities|Casting|CastToPlayerSave _returnvalue))
  (Variables|Default|SetPlayerSettings (Variables|/Game/Blueprints/AllLevels/PlayerSave.PlayerSave_C|GetS_PlayerInfo _asplayer_save)))

(fn MovePhase
  (params (MovementValue :type Integer))
  (bind _currentspace (Variables|Default|GetCurrentSpace))
  (Default|MovementCheck _currentspace MovementValue (LocalVariables|GetBlank) (LocalVariables|GetBlank2) true _currentspace "NewEnumerator0"))

(fn StartingDeck
  (bind _outactors (Actor|GetAllActorsOfClass "/Game/Blueprints/Cards/IndividualCards/00_Card.00_Card_C"))
  (bind _output_get (Variables|CardLocations|SetDeck (Utilities|Array|MakeArray (Utilities|Array|Get(acopy) _outactors) (Utilities|Array|Get(acopy) _outactors) (Utilities|Array|Get(acopy) _outactors 1) (Utilities|Array|Get(acopy) _outactors 1) (Utilities|Array|Get(acopy) _outactors 2) (Utilities|Array|Get(acopy) _outactors 2) (Utilities|Array|Get(acopy) _outactors 3) (Utilities|Array|Get(acopy) _outactors 4) (Utilities|Array|Get(acopy) _outactors 5))))
  (Utilities|Array|Shuffle _output_get)
  (for _index (range 1 (Variables|Default|GetStartingHandSize))
    (CardFunctions|Draw false)))

(fn Draw
  (params (MovePhase :type Boolean))
  (bind _asgameplay_gm (Utilities|GetGameplayGM))
  (bind _deck (Variables|CardLocations|GetDeck))
  (bind _output (Utilities|Array|Get(acopy) _deck))
  ;[1 1 1] If there's no draw pile, shuffle the discard into the draw.  If there's neither, than no draw is possible.
  (if (<= (Utilities|Array|Length _deck) 0)
    (bind _success (CardFunctions|ShuffleDiscard))
    (if _success
      _
      (else
        (return false))))
  ;[1 1 1] Pulls a card out of the draw pile and into the hand.  Updates the WB
  (LocalVariables|SetNewCard _output)
  (Utilities|Array|Add (Variables|CardLocations|GetHand) _output)
  (Utilities|Array|RemoveIndex (Variables|CardLocations|GetDeck))
  (Utilities|IsValid (Variables|Default|GetGameplayChatWB)
    (:Is%20Valid
      _)
    (:Is%20Not%20Valid
      (CallFunction|SetupChatWindow)))
  (Default|CollectHandData (Variables|Default|GetGameplayChatWB))
  ;[1 1 1] Checks if in combat, which overrides movement phase
  (bind _valid_ (Default|CheckforCurrentCom _asgameplay_gm))
  (if _valid_
    (CallFunction|SetTurnPhase "NewEnumerator4")
    (Default|ReturnCombat _asgameplay_gm)
    (return true)
    (else
      ;[1 1 1] If this card was drawn as part of the movement phase, than find the possible directions
      (if MovePhase
        (CallFunction|ServerDeterminePath (Variables|/Game/Blueprints/Cards/IndividualCards/00_Card.00_Card_C|GetMovement (LocalVariables|GetNewCard)))
        (Variables|Default|SetTurnPhase "NewEnumerator2")
        (return true)
        (else
          (return true))))))

(fn ShuffleDiscard
  (bind _discard (Variables|CardLocations|GetDiscard))
  ;[1 1 1] Move the Discard back into the Deck, clear the discard, and then shuffle. If the discard is empty, pass back a failure.
  (if (> (Utilities|Array|Length (Variables|CardLocations|GetDiscard)) 0)
    (bind _output_get (Variables|CardLocations|SetDeck _discard))
    (Utilities|Array|Clear _discard)
    (Utilities|Array|Shuffle _output_get)
    (return true)
    (else
      (return false))))

(fn PlayCard
  (params (CardNumber :type Integer))
  (Development|PrintString "Test")
  (LocalVariables|SetHandIndex CardNumber)
  (Utilities|Array|Add (Variables|CardLocations|GetDiscard) (Utilities|Array|Get(acopy) (Variables|CardLocations|GetHand) (LocalVariables|GetHandIndex)))
  (Utilities|Array|RemoveIndex (Variables|CardLocations|GetHand) (LocalVariables|GetHandIndex))
  (return true))

(fn SwitchTurnPhase
  (params (NewParam :type TurnPhases%20Enum :default "NewEnumerator0"))
  (Variables|Default|SetTurnPhase NewParam))

(fn DisplayTest
  (Utilities|FlowControl|Sequence))

(fn InitialTurnPhase
  (if (== (Variables|Default|GetCurrentTurn) (Variables|Default|GetTurnNumber))
    (Variables|Default|SetTurnPhase "NewEnumerator1")
    (else
      (Variables|Default|SetTurnPhase "NewEnumerator0"))))

(fn ResolveEndOfTurn
  (Variables|Default|SetTurnPhase "NewEnumerator0")
  (CallFunction|EndTurn))

(fn HandtoSelected
  (params (Position :type Integer))
  (Utilities|IsValid (Variables|CardLocations|GetSelectedCard)
    (:Is%20Valid
      (Utilities|Array|Add (Variables|CardLocations|GetHand) 0))
    (:Is%20Not%20Valid
      _))
  (Variables|CardLocations|SetSelectedCard (Utilities|Array|Get(acopy) (Variables|CardLocations|GetHand) Position))
  (Utilities|Array|RemoveIndex (Variables|CardLocations|GetHand) Position))

(fn SelectedtoHand
  (Utilities|IsValid (Variables|CardLocations|GetSelectedCard)
    (:Is%20Valid
      (Utilities|Array|Add (Variables|CardLocations|GetHand) (Variables|CardLocations|GetSelectedCard)))
    (:Is%20Not%20Valid
      _))
  (Variables|CardLocations|SetSelectedCard 0))

(fn SelectedtoAttack
  (Utilities|IsValid (Variables|CardLocations|GetSelectedCard)
    (:Is%20Valid
      (Variables|CardLocations|SetAttackCard (Variables|CardLocations|GetSelectedCard)))
    (:Is%20Not%20Valid
      _))
  (Variables|CardLocations|SetSelectedCard 0))

(fn SelectedtoBoth
  (Utilities|IsValid (Variables|CardLocations|GetSelectedCard)
    (:Is%20Valid
      (Variables|CardLocations|SetBothCard (Variables|CardLocations|GetSelectedCard)))
    (:Is%20Not%20Valid
      _))
  (Variables|CardLocations|SetSelectedCard 0))

(fn SelectedtoDefend
  (Utilities|IsValid (Variables|CardLocations|GetSelectedCard)
    (:Is%20Valid
      (Variables|CardLocations|SetDefenseCard (Variables|CardLocations|GetSelectedCard)))
    (:Is%20Not%20Valid
      _))
  (Variables|CardLocations|SetSelectedCard 0))

(fn AttacktoHand
  (Utilities|IsValid (Variables|CardLocations|GetAttackCard)
    (:Is%20Valid
      (Utilities|Array|Add (Variables|CardLocations|GetHand) (Variables|CardLocations|GetAttackCard)))
    (:Is%20Not%20Valid
      _))
  (Variables|CardLocations|SetAttackCard 0))

(fn BothtoHand
  (Utilities|IsValid (Variables|CardLocations|GetBothCard)
    (:Is%20Valid
      (Utilities|Array|Add (Variables|CardLocations|GetHand) (Variables|CardLocations|GetBothCard)))
    (:Is%20Not%20Valid
      _))
  (Variables|CardLocations|SetBothCard 0))

(fn DefensetoHand
  (Utilities|IsValid (Variables|CardLocations|GetDefenseCard)
    (:Is%20Valid
      (Utilities|Array|Add (Variables|CardLocations|GetHand) (Variables|CardLocations|GetDefenseCard)))
    (:Is%20Not%20Valid
      _))
  (Variables|CardLocations|SetDefenseCard 0))

(fn TakeDamage
  (params (IncomingDamage :type Integer))
  (bind _output_get (Variables|Default|SetInjuries (+ IncomingDamage (Variables|Default|GetInjuries))))
  (if (>= _output_get (Variables|Default|GetHitPoints))
    (CallFunction|ShufflesOffThisMortalCoil))
  (return (>= _output_get (Variables|Default|GetHitPoints))))

(fn ShufflesOffThisMortalCoil)

(fn SetMonsterCard
  (params (Current :type Array%20of%2000%20Monster%20Cards%20Object%20References))
  (Variables|Default|SetCurrentMonsterCard Current))

(event Custom|TestFunction
  (Default|EndTurn (Utilities|GetGameplayGM)))

(event Input|KeyboardEvents|2
  (params (Key :type Key%20Structure)))

(event Input|KeyboardEvents|SpaceBar
  (params (Key :type Key%20Structure))
  (:Pressed
    (switch Utilities|FlowControl|Switch|SwitchonTurnPhases (Variables|Default|GetTurnPhase)
      (:NewEnumerator0
        _)
      (:NewEnumerator5
        _))
    (Variables|Default|SetTurnPhase "NewEnumerator1")))

(event Input|KeyboardEvents|1
  (params (Key :type Key%20Structure))
  (:Pressed
    (CallFunction|TestFunction)))

(event Input|KeyboardEvents|3
  (params (Key :type Key%20Structure)))

(event Input|KeyboardEvents|4
  (params (Key :type Key%20Structure))
  (:Pressed
    (Variables|Default|SetTurnNumber 4)))

(event Custom|SetCurrentTurn
  (params (CurrentTurn :type Integer))
  (Variables|Default|SetCurrentTurn CurrentTurn))

(event Custom|SetTurnPhase
  (params (TurnPhase :type TurnPhases%20Enum :default "NewEnumerator0"))
  (Variables|Default|SetTurnPhase TurnPhase))

(event Custom|BonusDraw
  (params (Add :type Integer))
  (Variables|Default|SetBonusDraws Add))

(event Custom|SetTurnOrder
  (params (Num :type Integer))
  (Variables|Default|SetTurnNumber Num))

(event Custom|ServerPieceMove
  (Default|PieceMove (Utilities|GetGameplayGM)))

(event Custom|ServerDeterminePath
  (params (Movement :type Integer))
  (Default|DeterminePath (Utilities|GetGameplayGM) Movement))

(event Custom|ServerPieceMovementPath
  (params (MovementPath :type Array%20of%20Board%20Space%20Object%20References))
  (Default|PieceMovementPath (Utilities|GetGameplayGM) MovementPath))